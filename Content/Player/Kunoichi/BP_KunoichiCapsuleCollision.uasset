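; Kunoichi player Blueprint that fights with a claymore and can transform into a Wolf.
; On BeginPlay it attaches a spawned claymore to the right-hand socket, and attack inputs play melee montages.
; E spawns a Wolf at the pawn's transform, then destroys the claymore and Kunoichi and possesses the Wolf.
; TryHitSheep, not called here, sphere-traces at the sword socket to consume sheep with a Niagara explosion; zoom is unwired WIP.
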(event OnComponentBeginOverlap(CollisionComponent)
  (params (OverlappedComponent :type Primitive%20Component%20Object%20Reference) (OtherActor :type Actor%20Object%20Reference) (OtherComp :type Primitive%20Component%20Object%20Reference) (OtherBodyIndex :type Integer) (bFromSweep :type Boolean) (SweepResult :type Hit%20Result%20Structure%20%28by%20ref%29)))

(event Input|EnhancedActionEvents|EnhancedInputActionIA_Attack
  (params (ActionValue :type Boolean) (ElapsedSeconds :type Float%20%28double-precision%29) (TriggeredSeconds :type Float%20%28double-precision%29) (InputAction :type Input%20Action%20Object%20Reference :default "/Game/Input/IA_Attack.IA_Attack"))
  (Animation|Montage|PlayMontage (Variables|Default|GetSkeletalMesh) "/Game/Player/Animations/Standing_Melee_Attack_Horizontal_Montage.Standing_Melee_Attack_Horizontal_Montage"))

(event Input|EnhancedActionEvents|EnhancedInputActionIA_SpecialAttack
  (params (ActionValue :type Boolean) (ElapsedSeconds :type Float%20%28double-precision%29) (TriggeredSeconds :type Float%20%28double-precision%29) (InputAction :type Input%20Action%20Object%20Reference :default "/Game/Input/IA_SpecialAttack.IA_SpecialAttack"))
  (Animation|Montage|PlayMontage (Variables|Default|GetSkeletalMesh) "/Game/Player/Kunoichi/Animation/Standing_Melee_Combo_Attack_Ver__2_Montage.Standing_Melee_Combo_Attack_Ver__2_Montage"))

(event Input|EnhancedActionEvents|EnhancedInputActionIA_ZoomIn
  (params (ActionValue :type Boolean) (ElapsedSeconds :type Float%20%28double-precision%29) (TriggeredSeconds :type Float%20%28double-precision%29) (InputAction :type Input%20Action%20Object%20Reference :default "/Game/Input/IA_ZoomIn.IA_ZoomIn"))
  ;[0.15 0.15 0.15 0.5] WIP ZoomIN/OUT
)

(event Input|EnhancedActionEvents|EnhancedInputActionIA_ZoomOut
  (params (ActionValue :type Boolean) (ElapsedSeconds :type Float%20%28double-precision%29) (TriggeredSeconds :type Float%20%28double-precision%29) (InputAction :type Input%20Action%20Object%20Reference :default "/Game/Input/IA_ZoomOut.IA_ZoomOut"))
  ;[0.15 0.15 0.15 0.5] WIP ZoomIN/OUT
)

(event EventBeginPlay
  (bind _returnvalue (Game|SpawnActorfromClass "/Game/Player/Weapons/BP_Claymore.BP_Claymore_C" (Transformation|GetSocketTransform (Variables|Default|GetSkeletalMesh) "RightHandWeaponSocket" "RTS_World") "Undefined" "MultiplyWithRoot" 0 0))
  (Transformation|AttachComponentToComponent _returnvalue (Variables|Default|GetSkeletalMesh) "RightHandWeaponSocket" "SnapToTarget" "SnapToTarget" "SnapToTarget" true))

(event Collision|EventActorBeginOverlap
  (params (OtherActor :type Actor%20Object%20Reference)))

(event EventTick
  (params (DeltaSeconds :type Float%20%28single-precision%29)))

(event Input|KeyboardEvents|E
  (params (Key :type Key%20Structure :default "None"))
  ;[0.15 0.15 0.15 0.5] Spawning Wolf at the same place as Kunoichi
  (:Pressed
    (bind _returnvalue (Game|SpawnActorfromClass "/Game/Player/Wolf.Wolf_C" (Transformation|GetActorTransform (Pawn|GetControlledPawn (Game|GetPlayerController 0))) "Undefined" "MultiplyWithRoot" 0 0))
    ;[0.15 0.15 0.15 0.5] Destroying Kunoichi Sword
    (for _array_element (Actor|GetAttachedActors (Pawn|GetControlledPawn (Game|GetPlayerController 0)) true false)
      (bind _asbp_claymore (Utilities|Casting|CastToBP_Claymore _array_element))
      (Actor|DestroyActor _asbp_claymore)
      ;[0.15 0.15 0.15 0.5] Destroying Kunoichi
      (Actor|DestroyActor (Pawn|GetControlledPawn (Game|GetPlayerController 0)))
      ;[0.15 0.15 0.15 0.5] Setting Wolf as current player
      (Pawn|Possess (Game|GetPlayerController 0) _returnvalue))))

(fn ConstructionScript)

(fn TryHitSheep
  (bind _skeletalmesh (Variables|Default|GetSkeletalMesh))
  (bind _returnvalue (Transformation|GetSocketLocation _skeletalmesh "Sword_joint"))
  (bind (_outhit _returnvalue_2) (Class|KismetSystemLibrary|SphereTraceSinglebyProfile _returnvalue _returnvalue 2e+02 "Vehicle" false 0 "None" true))
  (if _returnvalue_2
    (bind _returnvalue_3 (Class|UWPlayerPawn|ConsumeSheep (.HitActor (Collision|BreakHitResult _outhit))))
    (if _returnvalue_3
      (Niagara|SpawnSystematLocation "/Game/MsvFx_Niagara_Explosion_Pack_01/Prefabs/Niagara_Explosion_03.Niagara_Explosion_03" (Transformation|GetSocketLocation (Variables|Default|GetSkeletalMesh) "Sword_joint")))))