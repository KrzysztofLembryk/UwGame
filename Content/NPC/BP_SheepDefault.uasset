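; BP_SheepDefault is a sheep NPC Blueprint that tints its body to reflect its current SheepPoints.
; On BeginPlay it creates a dynamic instance of M_SheepBody on the Body component and applies the initial color.
; SetColor maps points to the red channel of SheepBaseColor and reruns whenever points change.
; The alone-state event is empty, with its color-switch logic left disconnected.
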(event Custom|SetColor
  (params (SheepValue :type Integer))
  (bind _sheepbodymaterialinstance (Variables|Default|GetSheepBodyMaterialInstance))
  (if (Utilities|IsValid _sheepbodymaterialinstance)
    (Rendering|Material|SetVectorParameterValue _sheepbodymaterialinstance "SheepBaseColor" (Math|Color|MakeColor (Math|Float|MapRangeClamped (Math|Conversions|ToFloat(Integer) SheepValue) 1.0 1e+01 0.0 1.0) 0.5 0.2) :!class /Script/Engine.MaterialInstanceDynamic)))

(event EventBeginPlay
  (bind _returnvalue (Rendering|Material|CreateDynamicMaterialInstance (Variables|Default|GetBody) 0 "/Game/Materials/M_SheepBody.M_SheepBody" "None" :!class /Script/Engine.PrimitiveComponent))
  (Variables|Default|SetSheepBodyMaterialInstance _returnvalue)
  (CallFunction|SetColor (Variables|Default|GetSheepPoints)))

(event Collision|EventActorBeginOverlap
  (params (OtherActor :type Actor%20Object%20Reference)))

(event EventTick
  (params (DeltaSeconds :type Float%20%28single-precision%29)))

(event EventOnSheepAloneStateChange
  (params (bInIsAlone :type Boolean)))

(event EventOnSheepPointsChanged
  (params (NewValue :type Integer))
  (CallFunction|SetColor NewValue))

(fn ConstructionScript)