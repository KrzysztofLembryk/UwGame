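; Kunoichi player Blueprint that spawns a claymore into the right-hand socket and fights sheep with melee attacks.
; Attack and special-attack inputs each play their own melee montage.
; TryHitSheep, not called within this file, sphere-traces at the sword joint, passes the hit actor to ConsumeSheep and spawns a Niagara explosion on success.
; The collision overlap event is empty, leaving its ConsumeSheep and delay nodes unconnected.
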(event OnComponentBeginOverlap(CollisionComponent)
  (params (OverlappedComponent :type Primitive%20Component%20Object%20Reference) (OtherActor :type Actor%20Object%20Reference) (OtherComp :type Primitive%20Component%20Object%20Reference) (OtherBodyIndex :type Integer) (bFromSweep :type Boolean) (SweepResult :type Hit%20Result%20Structure%20%28by%20ref%29)))

(event Input|EnhancedActionEvents|EnhancedInputActionIA_Attack
  (params (ActionValue :type Boolean) (ElapsedSeconds :type Float%20%28double-precision%29) (TriggeredSeconds :type Float%20%28double-precision%29) (InputAction :type Input%20Action%20Object%20Reference :default "/Game/Input/IA_Attack.IA_Attack"))
  (Animation|Montage|PlayMontage (Variables|Default|GetSkeletalMesh) "/Game/Player/Animations/Standing_Melee_Attack_Horizontal_Montage.Standing_Melee_Attack_Horizontal_Montage"))

(event Input|EnhancedActionEvents|EnhancedInputActionIA_SpecialAttack
  (params (ActionValue :type Boolean) (ElapsedSeconds :type Float%20%28double-precision%29) (TriggeredSeconds :type Float%20%28double-precision%29) (InputAction :type Input%20Action%20Object%20Reference :default "/Game/Input/IA_SpecialAttack.IA_SpecialAttack"))
  (Animation|Montage|PlayMontage (Variables|Default|GetSkeletalMesh) "/Game/Player/Kunoichi/Animation/Standing_Melee_Combo_Attack_Ver__2_Montage.Standing_Melee_Combo_Attack_Ver__2_Montage"))

(event EventBeginPlay
  (bind _returnvalue (Game|SpawnActorfromClass "/Game/Player/Weapons/BP_Claymore.BP_Claymore_C" (Transformation|GetSocketTransform (Variables|Default|GetSkeletalMesh) "RightHandWeaponSocket" "RTS_World") "Undefined" "MultiplyWithRoot" 0 0))
  (Transformation|AttachComponentToComponent _returnvalue (Variables|Default|GetSkeletalMesh) "RightHandWeaponSocket" "SnapToTarget" "SnapToTarget" "SnapToTarget" true))

(event Collision|EventActorBeginOverlap
  (params (OtherActor :type Actor%20Object%20Reference)))

(event EventTick
  (params (DeltaSeconds :type Float%20%28single-precision%29)))

(fn ConstructionScript)

(fn TryHitSheep
  (bind _skeletalmesh (Variables|Default|GetSkeletalMesh))
  (bind _returnvalue (Transformation|GetSocketLocation _skeletalmesh "Sword_joint"))
  (bind (_outhit _returnvalue_2) (Class|KismetSystemLibrary|SphereTraceSinglebyProfile _returnvalue _returnvalue 2e+02 "Vehicle" false 0 "None" true))
  (if _returnvalue_2
    (bind _returnvalue_3 (Class|UWPlayerPawn|ConsumeSheep (.HitActor (Collision|BreakHitResult _outhit))))
    (if _returnvalue_3
      (Niagara|SpawnSystematLocation "/Game/MsvFx_Niagara_Explosion_Pack_01/Prefabs/Niagara_Explosion_03.Niagara_Explosion_03" (Transformation|GetSocketLocation (Variables|Default|GetSkeletalMesh) "Sword_joint")))))